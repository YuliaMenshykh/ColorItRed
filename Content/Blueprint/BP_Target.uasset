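; BP_Target is a wandering, jumping pawn that works as an infectable tag target, switching between yellow and red.
; Tick uses a random Delay to pace jumps and AI moves to random reachable points nearby.
; Hits from BP_Player or red targets turn it red, while a non-red BP_Cleaner restores yellow, with state read from material names.
; Each change adjusts the game mode's IsTargetRed counter, which falls on red and rises on yellow.
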(event Collision|EventHit
  (params (MyComp :type Primitive%20Component%20Object%20Reference) (Other :type Actor%20Object%20Reference) (OtherComp :type Primitive%20Component%20Object%20Reference) (bSelfMoved :type Boolean) (HitLocation :type Vector :default "0, 0, 0") (HitNormal :type Vector :default "0, 0, 0") (NormalImpulse :type Vector :default "0, 0, 0") (Hit :type Hit%20Result%20Structure%20%28by%20ref%29))
  (bind _cube (Variables|Default|GetCube))
  (bind _returnvalue (Rendering|Material|GetMaterial _cube 0))
  (bind _returnvalue_2 (Utilities|GetObjectName _returnvalue))
  (bind _returnvalue_3 (== _returnvalue_2 "Yellow"))
  (Utilities|Casting|CastToBP_Player Other
    (:then
      (if _returnvalue_3
        (Utilities|FlowControl|Sequence
          (:then_0
            (Rendering|Material|SetMaterial (Variables|Default|GetCube) 0 "/Game/Materials/Red.Red")
            (Utilities|FlowControl|DoOnce false :!label _label
              (:Completed
                (Audio|PlaySoundatLocation "/Game/StarterContent/Audio/interface-124464.interface-124464" HitLocation "0, 0, 0" 1.0 1.0 0.0 0 0 0 0)
                (bind _asbp_game_mode (Utilities|Casting|CastToBP_GameMode (Game|GetGameMode)))
                (Variables|/Game/Blueprint/BP_GameMode.BP_GameMode_C|SetIsTargetRed? _asbp_game_mode (- (Variables|/Game/Blueprint/BP_GameMode.BP_GameMode_C|GetIsTargetRed? _asbp_game_mode) 1)))))
          (:then_1
            (goto _label Reset)))))
    (:CastFailed
      (bind _asbp_target (Utilities|Casting|CastToBP_Target Other)
        (:then
          (if (and (== (Utilities|GetObjectName (Rendering|Material|GetMaterial (Variables|BP_Target_C|GetCube _asbp_target) 0)) "Red") _returnvalue_3)
            (Utilities|FlowControl|Sequence
              (:then_0
                (Rendering|Material|SetMaterial (Variables|Default|GetCube) 0 "/Game/Materials/Red.Red")
                (Utilities|FlowControl|DoOnce false :!label _label_2
                  (:Completed
                    (bind _asbp_game_mode_2 (Utilities|Casting|CastToBP_GameMode (Game|GetGameMode)))
                    (Variables|/Game/Blueprint/BP_GameMode.BP_GameMode_C|SetIsTargetRed? _asbp_game_mode_2 (- (Variables|/Game/Blueprint/BP_GameMode.BP_GameMode_C|GetIsTargetRed? _asbp_game_mode_2) 1)))))
              (:then_1
                (goto _label_2 Reset)))))
        (:CastFailed
          (bind _asbp_cleaner (Utilities|Casting|CastToBP_Cleaner Other))
          (if (and (!= (Utilities|GetObjectName (Rendering|Material|GetMaterial (Variables|/Game/Blueprint/BP_Cleaner.BP_Cleaner_C|GetCube _asbp_cleaner) 0)) "Red") (== (Utilities|GetObjectName (Rendering|Material|GetMaterial (Variables|Default|GetCube) 0)) "Red"))
            (Utilities|FlowControl|Sequence
              (:then_0
                (Rendering|Material|SetMaterial (Variables|Default|GetCube) 0 "/Game/Materials/Yellow.Yellow")
                (Utilities|FlowControl|DoOnce false :!label _label_3
                  (:Completed
                    (bind _asbp_game_mode_3 (Utilities|Casting|CastToBP_GameMode (Game|GetGameMode)))
                    (Variables|/Game/Blueprint/BP_GameMode.BP_GameMode_C|SetIsTargetRed? _asbp_game_mode_3 (+ (Variables|/Game/Blueprint/BP_GameMode.BP_GameMode_C|GetIsTargetRed? _asbp_game_mode_3) 1)))))
              (:then_1
                (goto _label_3 Reset)))))))))

(event EventTick
  (params (DeltaSeconds :type Float%20%28single-precision%29))
  ;[1 1 1] Movement
  (Utilities|FlowControl|Delay (Math|Random|RandomFloatinRange 1.0 3.0))
  (Variables|Default|SetIsMoving true)
  (Character|Jump)
  (AI|AIMoveTo self (.RandomLocation (AI|Navigation|GetRandomReachablePointinRadius (Transformation|GetActorLocation) 1e+03 0 0)) 0 5.0 false
    (:OnSuccess
      _)
    (:OnFail
      _))
  (Variables|Default|SetIsMoving false)
  (Character|Jump))

(fn ConstructionScript
  (|CallParentFunction))