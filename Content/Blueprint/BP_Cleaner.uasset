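; BP_Cleaner is a wandering character that turns red when the player collides with it.
; A delayed Tick repeatedly sends it to random reachable nearby points with AI MoveTo, and it jumps when each move succeeds or fails.
; The first player hit also plays a sound and decrements BP_GameMode's IsCleanerRed counter, guarded by DoOnce.
; A spark emitter node is present but unconnected.
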(event EventBeginPlay)

(event Collision|EventHit
  (params (MyComp :type Primitive%20Component%20Object%20Reference) (Other :type Actor%20Object%20Reference) (OtherComp :type Primitive%20Component%20Object%20Reference) (bSelfMoved :type Boolean) (HitLocation :type Vector :default "0, 0, 0") (HitNormal :type Vector :default "0, 0, 0") (NormalImpulse :type Vector :default "0, 0, 0") (Hit :type Hit%20Result%20Structure%20%28by%20ref%29))
  ;[1 1 1] On hit event
  (Utilities|Casting|CastToBP_Player Other)
  (Rendering|Material|SetMaterial (Variables|Components|GetCube) 0 "/Game/Materials/Red.Red")
  (Utilities|FlowControl|DoOnce false
    (:Completed
      (Audio|PlaySoundatLocation "/Game/StarterContent/Audio/shooting-sound-fx-159024.shooting-sound-fx-159024" HitLocation "0, 0, 0" 1.0 1.0 0.0 0 0 0 0)
      (bind _asbp_game_mode (Utilities|Casting|CastToBP_GameMode (Game|GetGameMode)))
      (Variables|/Game/Blueprint/BP_GameMode.BP_GameMode_C|SetIsCleanerRed? _asbp_game_mode (- (Variables|/Game/Blueprint/BP_GameMode.BP_GameMode_C|GetIsCleanerRed? _asbp_game_mode) 1)))))

(event EventTick
  (params (DeltaSeconds :type Float%20%28single-precision%29))
  ;[1 1 1] Moving
  (Utilities|FlowControl|Delay (Math|Random|RandomFloatinRange 1.0 3.0))
  (Variables|Default|SetIsMoving? true)
  (AI|AIMoveTo self (.RandomLocation (AI|Navigation|GetRandomReachablePointinRadius (Transformation|GetActorLocation) 1e+03 0 0)) 0 5.0 false
    (:OnSuccess
      _)
    (:OnFail
      _))
  (Variables|Default|SetIsMoving? false)
  (Character|Jump))

(fn ConstructionScript)