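; BP_EnemySpawner is a spawner actor that populates its surroundings with targets and cleaners when play begins.
; On BeginPlay it spawns a random number of BP_Target actors, then a smaller random batch of BP_Cleaner actors.
; Spawn positions come from random reachable navigation points around the spawner, with a fixed height and random yaw.
; It then creates the AmountOfCleaners widget and adds it to the viewport.
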(event EventBeginPlay
  (bind _returnvalue (Transformation|GetActorLocation))
  (bind _returnvalue_2 (Transformation|GetActorLocation))
  (bind _randomlocation (AI|Navigation|GetRandomReachablePointinRadius _returnvalue 1.5e+03 0 0))
  (bind _randomlocation_2 (AI|Navigation|GetRandomReachablePointinRadius _returnvalue_2 1.5e+03 0 0))
  (for _index (range 0 (Math|Random|RandomIntegerinRange 2 9))
    (Game|SpawnActorfromClass "/Game/Blueprint/BP_Target.BP_Target_C" (Math|Transform|MakeTransform (Math|Vector|MakeVector (.x _randomlocation) (.y _randomlocation) 5e+01) (Math|Rotator|MakeRotator 0.0 0.0 (.yaw (Math|Random|RandomRotator false))) "1.000000,1.000000,1.000000") "Undefined" "MultiplyWithRoot" 0 0))
  (for _index_2 (range 0 (Math|Random|RandomIntegerinRange 2 4))
    (Game|SpawnActorfromClass "/Game/Blueprint/BP_Cleaner.BP_Cleaner_C" (Math|Transform|MakeTransform (Math|Vector|MakeVector (.x _randomlocation_2) (.y _randomlocation_2) 5e+01) (Math|Rotator|MakeRotator 0.0 0.0 (.yaw (Math|Random|RandomRotator false))) "1.000000,1.000000,1.000000") "Undefined" "MultiplyWithRoot" 0 0))
  (bind _returnvalue_3 (UserInterface|CreateWidget "/Game/Menus/AmountOfCleaners.AmountOfCleaners_C"))
  (UserInterface|Viewport|AddtoViewport _returnvalue_3 0))

(fn ConstructionScript)